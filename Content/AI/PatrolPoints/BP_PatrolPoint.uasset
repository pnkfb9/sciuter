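; BP_PatrolPoint is an AI patrol waypoint that links to next and previous points and visualizes those links as splines.
; Its construction script totals the links, clears the Cube's child components and calls DrawSplines for each direction with its own color.
; DrawSplines adds a spline per linked point, attached to this Cube and running to that point's Cube.
; Opposite right and forward offsets keep the two directions visually apart.
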(fn ConstructionScript
  (LocalVariables|SettotPoints (+ (Utilities|Array|Length (Variables|Default|GetnextPoints)) (Utilities|Array|Length (Variables|Default|GetprevPoints))))
  (for _array_element (Components|GetChildrenComponents (Variables|Default|GetCube) false)
    (Components|DestroyComponent _array_element))
  ;[1 1 1] draw the splines for forward and backward direction
  (CallFunction|DrawSplines (Variables|Default|GetnextPoints) -2e+01 "(R=0.005959,G=0.000000,B=0.870000,A=1.000000)")
  (CallFunction|DrawSplines (Variables|Default|GetprevPoints) 2e+01 "(R=0.490000,G=0.070479,B=0.000000,A=1.000000)"))

(fn DrawSplines
  (params (points :type Array%20of%20BP%20Patrol%20Point%20Object%20References) (betweenLines :type Float%20%28double-precision%29) (splineColor :type Linear%20Color%20Structure))
  (bind _cube (Variables|Default|GetCube))
  (bind _cube_2 (Variables|Default|GetCube))
  (for _array_element points
    (bind _output_get (LocalVariables|SetcurrentPoint _array_element))
    ;[1 1 1] add spline component
    (bind _returnvalue (AddComponent|AddSplineComponent _output_get false))
    (bind _output_get_2 (LocalVariables|SetcurrentSpline _returnvalue))
    (Transformation|AttachComponentToComponent _output_get_2 (Variables|Default|GetCube) "None" "SnapToTarget" "KeepRelative" "KeepRelative" true)
    (Class|SplineComponent|SetUnselectedSplineSegmentColor (LocalVariables|GetcurrentSpline) splineColor)
    ;[1 1 1] set start point of spline
    (Spline|SetLocationatSplinePoint (LocalVariables|GetcurrentSpline) 0 (+ (Transformation|GetWorldLocation _cube_2) (* (Math|Vector|GetRightVector _cube_2) betweenLines) (* (Math|Vector|GetForwardVector _cube_2) betweenLines)) "World" false)
    ;[1 1 1] set end point of spline
    (Spline|SetLocationatSplinePoint (LocalVariables|GetcurrentSpline) 1 (+ (Transformation|GetWorldLocation (Variables|BP_PatrolPoint_C|GetCube (LocalVariables|GetcurrentPoint))) (* (Math|Vector|GetRightVector _cube) betweenLines) (* (Math|Vector|GetForwardVector _cube) betweenLines)) "World" true)))